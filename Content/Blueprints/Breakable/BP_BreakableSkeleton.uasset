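; BP_BreakableSkeleton is a breakable skeleton actor built on a Chaos geometry collection and a capsule.
; GetHit runs the parent's hit logic, then plays the break sound at the impact point.
; On a Chaos break event, it sets a short lifespan, makes the capsule ignore pawns and turns off further break notifications.
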(event OnChaosBreakEvent(GeometryCollection)
  (params (BreakEvent :type Chaos%20Break%20Event%20Structure%20%28by%20ref%29))
  (Actor|SetLifeSpan 3.0)
  (Collision|SetCollisionResponsetoChannel (Variables|Default|GetCapsule) "ECC_Pawn" "ECR_Ignore")
  (Class|GeometryCollectionComponent|SetNotifyBreaks (Variables|Default|GetGeometryCollection) false))

(event EventBeginPlay)

(event Collision|EventActorBeginOverlap
  (params (OtherActor :type Actor%20Object%20Reference)))

(event EventTick
  (params (DeltaSeconds :type Float%20%28single-precision%29)))

(event EventGetHit
  (params (Hit :type Hit%20Result%20Structure%20%28by%20ref%29) (Hitter :type Actor%20Object%20Reference))
  (|CallParentFunction Hit Hitter)
  (Audio|PlaySoundatLocation (Variables|Default|GetBreakSound) (.ImpactPoint (Collision|BreakHitResult Hit)) "0, 0, 0" 1.0 1.0 0.0 0 0 0 0))

(fn ConstructionScript)
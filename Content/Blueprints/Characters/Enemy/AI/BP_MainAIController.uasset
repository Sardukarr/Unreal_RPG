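; Enemy AI controller that turns perception of the player into a combat target on the Blackboard.
; Possession sets the enemy state to Idle, and each perception update looks for the player and caches its stimuli.
; The first sense sets or clears the combat target, while the second only sets it.
; Tick and per-target perception handlers check stimuli but do nothing.
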(event OnPerceptionUpdated(AIPerception)
  (params (UpdatedActors :type Array%20of%20Actor%20Object%20References))
  (bind (_perceptioninfo _bisfound _returnvalue) (Class|MainAIController|FindPlayerinActors UpdatedActors))
  (if _bisfound
    (Variables|Default|SetPlayerSeen _returnvalue)
    (bind _output_get (Variables|Default|SetPerception%20Info _perceptioninfo))
    (bind (_array_element _array_index) (Utilities|Array|ForEachLoopwithBreak (.LastSensedStimuli (Utilities|Struct|BreakActorPerceptionBlueprintInfo _output_get)))
      (:LoopBody
        (Variables|Default|SetLastStimulus _array_element)
        (switch int _array_index
          (:0
            (if (.bSuccessfullySensed (Utilities|Struct|BreakAIStimulus (Variables|Default|GetLastStimulus)))
              (AI|Components|Blackboard|SetValueasObject (Variables|Default|GetBlackboard) (Variables|Blackboard|GetCombatTargetBlackboard) (Variables|Default|GetPlayerSeen))
              (else
                (AI|Components|Blackboard|SetValueasObject (Variables|Default|GetBlackboard) (Variables|Blackboard|GetCombatTargetBlackboard) 0))))
          (:1
            (if (.bSuccessfullySensed (Utilities|Struct|BreakAIStimulus (Variables|Default|GetLastStimulus)))
              (AI|Components|Blackboard|SetValueasObject (Variables|Default|GetBlackboard) (Variables|Blackboard|GetCombatTargetBlackboard) (Variables|Default|GetPlayerSeen)))))))))

(event OnTargetPerceptionInfoUpdated(AIPerception)
  (params (UpdateInfo :type Actor%20Perception%20Update%20Info%20Structure%20%28by%20ref%29))
  (if (.bSuccessfullySensed (Utilities|Struct|BreakAIStimulus (.Stimulus (Utilities|Struct|BreakActorPerceptionUpdateInfo UpdateInfo))))
    _))

(event EventBeginPlay
  (|CallParentFunction))

(event EventPossess
  (params (PossessedPawn :type Pawn%20Object%20Reference))
  (|CallParentFunction PossessedPawn)
  (AI|Components|Blackboard|SetValueasEnum (Variables|Default|GetBlackboard) (Variables|Blackboard|GetEnemyStateBlackboard) (Utilities|Enum|LiteralenumEEnemyState "EES_Idle")))

(event EventTick
  (params (DeltaSeconds :type Float%20%28single-precision%29))
  (|CallParentFunction DeltaSeconds)
  (if (Utilities|IsValid (Variables|Default|GetPlayerSeen))
    (if (.bSuccessfullySensed (Utilities|Struct|BreakAIStimulus (Utilities|Array|Get(acopy) (.LastSensedStimuli (Utilities|Struct|BreakActorPerceptionBlueprintInfo (Variables|Default|GetPerception%20Info))))))
      _)))

(fn ConstructionScript)
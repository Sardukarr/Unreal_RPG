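; BP_Weapon is a weapon item Blueprint that can trigger physics force fields at a given location.
; Its CreateForceFields event casts the child actor of its FieldSystemActor component to BP_FieldWeaponSystem and passes the location to TriggerField.
; A disconnected debug box trace between the BoxTraceStart and BoxTraceEnd components never runs, and BeginPlay, Tick and the construction script are empty.
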(event EventBeginPlay)

(event EventCreateForceFields
  (params (FieldLocation :type Vector%20%28by%20ref%29 :default "0, 0, 0"))
  (bind _asbp_field_weapon_system (Utilities|Casting|CastToBP_FieldWeaponSystem (Variables|/Script/Engine.ChildActorComponent|GetChildActor (Variables|Default|GetFieldSystemActor))))
  (Default|TriggerField _asbp_field_weapon_system FieldLocation))

(event EventTick
  (params (DeltaSeconds :type Float%20%28single-precision%29)))

(fn ConstructionScript)